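; FG_Camera is a camera actor that frames the player's SideScrollerCharacter and the Varon_Nandur actor in a side-on view.
; After a short delay at BeginPlay, it caches both references.
; Each tick, it keeps its X and moves to their Y midpoint, with Z set from a slightly raised average of their heights.
; A distance-based, clamped field-of-view zoom is present but disconnected, so it never runs.
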(event `self.ReceiveBeginPlay`
  (`KismetSystemLibrary.Delay` 0.03)
  (bind _asside_scroller_character (cast `/Game/SideScrollerBP/Blueprints/SideScrollerCharacter` (`GameplayStatics.GetPlayerCharacter` 0)))
  (set `self.As Side Scroller Character` _asside_scroller_character)
  (bind _returnvalue (`GameplayStatics.GetActorOfClass` "/Game/Varon_Nandur/Varon_Nandur.Varon_Nandur_C"))
  (bind _output_get (set `self.Varon_Nandur` _returnvalue))
  (cast `/Game/Varon_Nandur/Varon_Nandur` _output_get))

(event `self.ReceiveTick`
  (params (DeltaSeconds :type "Float (single-precision)"))
  (bind _as_side_scroller_character (`self.As Side Scroller Character`))
  (bind _varon_nandur (`self.Varon_Nandur`))
  (if (and (`KismetSystemLibrary.IsValid` _as_side_scroller_character) (`KismetSystemLibrary.IsValid` _varon_nandur))
    (`self.K2_SetActorLocation` (`KismetMathLibrary.MakeVector` (.x (`self.K2_GetActorLocation`)) (/ (+ (.y (`self.K2_GetActorLocation` _as_side_scroller_character)) (.y (`self.K2_GetActorLocation` _varon_nandur))) 2.0) (/ (+ (.z (`self.K2_GetActorLocation` _as_side_scroller_character)) (.z (`self.K2_GetActorLocation` _varon_nandur))) 1.7)))))

(fn `UserConstructionScript`)